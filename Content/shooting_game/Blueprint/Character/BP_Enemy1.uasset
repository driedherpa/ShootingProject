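; BP_Enemy1 is a shooting-game enemy that moves at a set speed along a local direction each tick.
; Incoming damage drains its health; at zero it snaps to its skeletal mesh's location, spawns an explosion effect and destroys itself.
; Overlapping BP_Fighter with its sphere deals contact damage to the fighter, then destroys the enemy with a scaled-down explosion.
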(event `self.ReceiveTick`
  (params (DeltaSeconds :type "Float (single-precision)"))
  (`self.K2_AddActorLocalOffset` (* (* DeltaSeconds (`self.EnemyMovementSpeed`)) (`self.Direction`))))

(event `self.ReceiveAnyDamage`
  (params (Damage :type "Float (single-precision)") (DamageType :type "DamageType Object Reference") (InstigatedBy :type "Controller Object Reference") (DamageCauser :type "Actor Object Reference"))
  (bind _output_get (set `self.Health` (- (`self.Health`) Damage)))
  (if (<= _output_get 0.0)
    (`self.K2_SetActorLocation` (`SceneComponent.K2_GetComponentLocation` (`self.SkeletalMesh`)))
    (`NiagaraFunctionLibrary.SpawnSystemAtLocation` "/Game/shooting_game/FX/VFX_EnemyExplosion1.VFX_EnemyExplosion1" (`self.K2_GetActorLocation`))
    (`self.K2_DestroyActor`)))

(event `self.Sphere.OnComponentBeginOverlap`
  (params (OverlappedComponent :type "PrimitiveComponent Object Reference") (OtherActor :type "Actor Object Reference") (OtherComp :type "PrimitiveComponent Object Reference") (OtherBodyIndex :type Integer) (bFromSweep :type Boolean) (SweepResult :type "HitResult Structure (by ref)"))
  (cast `/Game/shooting_game/Blueprint/Character/BP_Fighter` OtherActor)
  (`GameplayStatics.ApplyDamage` OtherActor (`self.EnemyDamage`))
  (`NiagaraFunctionLibrary.SpawnSystemAtLocation` "/Game/shooting_game/FX/VFX_EnemyExplosion1.VFX_EnemyExplosion1" (`self.K2_GetActorLocation`) (struct) (0.4 0.4 0.4))
  (`self.K2_DestroyActor`))

(fn `UserConstructionScript`)