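; BP_Fighter is the player fighter in a shooting game, handling movement, shooting, health and game over.
; Enhanced Input drives movement along local Y and looping timers that spawn bullets or bombs while held; only bullets also fire immediately on press.
; Damage reduces health, exposed through getters; at zero it explodes, hides, then shows WBP_GameOver and switches to the menu input mapping.
; A restart input reloads Level1.
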(event `self.ReceiveBeginPlay`
  (`EnhancedInputSubsystemInterface.AddMappingContext` (pcsubsystem `EnhancedInputLocalPlayerSubsystem` (`GameplayStatics.GetPlayerController` 0)) "/Game/shooting_game/Input/IMC_Fighter.IMC_Fighter" 0 (struct))
  (set `self.PlayerHealth` 100.0)
  (bind _returnvalue (`|CreateWidget` "/Game/shooting_game/UI/WBP_UI.WBP_UI_C"))
  (`UserWidget.AddToViewport` _returnvalue 0))

(event `EnhancedInput|/Game/shooting_game/Input/IA_FighterMove`
  (params (ActionValue :type "Float (double-precision)") (ElapsedSeconds :type "Float (double-precision)") (TriggeredSeconds :type "Float (double-precision)") (InputAction :type "InputAction Object Reference" :default "/Game/shooting_game/Input/IA_FighterMove.IA_FighterMove"))
  (:`Triggered`
    (`self.K2_AddActorLocalOffset` (`KismetMathLibrary.MakeVector` 0.0 (* ActionValue (`self.MovementSpeed`))))))

(event `ShootingBullet`
  (`|SpawnActorFromClass` "/Game/shooting_game/Blueprint/SubObject/BP_Bullet.BP_Bullet_C" (`SceneComponent.K2_GetComponentToWorld` (`self.DefaultSceneRoot`)) "Undefined" "MultiplyWithRoot" null null))

(event `EnhancedInput|/Game/shooting_game/Input/IA_Shoot`
  (params (ActionValue :type Boolean) (ElapsedSeconds :type "Float (double-precision)") (TriggeredSeconds :type "Float (double-precision)") (InputAction :type "InputAction Object Reference" :default "/Game/shooting_game/Input/IA_Shoot.IA_Shoot"))
  (:`Started`
    (`self.ShootingBullet`)
    (bind _returnvalue (`KismetSystemLibrary.K2_SetTimerDelegate` (delegate `ShootingBullet`) (`self.ShootRate`) true))
    (set `self.ShootCheck` _returnvalue))
  (:`Completed`
    (`KismetSystemLibrary.K2_ClearAndInvalidateTimerHandle` (`self.ShootCheck`))))

(event `ShootingBomb`
  (`|SpawnActorFromClass` "/Game/shooting_game/Blueprint/SubObject/BP_BulletBomb.BP_BulletBomb_C" (`SceneComponent.K2_GetComponentToWorld` (`self.DefaultSceneRoot`)) "Undefined" "MultiplyWithRoot" null null))

(event `EnhancedInput|/Game/shooting_game/Input/IA_ShootBomb`
  (params (ActionValue :type Boolean) (ElapsedSeconds :type "Float (double-precision)") (TriggeredSeconds :type "Float (double-precision)") (InputAction :type "InputAction Object Reference" :default "/Game/shooting_game/Input/IA_ShootBomb.IA_ShootBomb"))
  (:`Started`
    (bind _returnvalue (`KismetSystemLibrary.K2_SetTimerDelegate` (delegate `ShootingBomb`) (`self.BombShootRate`) true))
    (set `self.BombShootCheck` _returnvalue))
  (:`Completed`
    (`KismetSystemLibrary.K2_ClearAndInvalidateTimerHandle` (`self.BombShootCheck`))))

(event `self.ReceiveTick`
  (params (DeltaSeconds :type "Float (single-precision)"))
  (set `self.LastVaildLocation` (`self.K2_GetActorLocation`)))

(event `self.ReceiveAnyDamage`
  (params (Damage :type "Float (single-precision)") (DamageType :type "DamageType Object Reference") (InstigatedBy :type "Controller Object Reference") (DamageCauser :type "Actor Object Reference"))
  (bind _output_get (set `self.PlayerHealth` (- (`self.PlayerHealth`) Damage)))
  (if (<= _output_get 0.0)
    (`NiagaraFunctionLibrary.SpawnSystemAtLocation` "/Game/shooting_game/FX/VFX_EnemyExplosion1.VFX_EnemyExplosion1" (`self.K2_GetActorLocation`))
    (`self.SetActorHiddenInGame` true)
    (`PrimitiveComponent.SetCollisionEnabled` (`self.Capsule`) "NoCollision")
    (`KismetSystemLibrary.Delay` 1.0)
    (`self.DieEvnet`)))

(event `EnhancedInput|/Game/shooting_game/Input/IA_Restart`
  (params (ActionValue :type Boolean) (ElapsedSeconds :type "Float (double-precision)") (TriggeredSeconds :type "Float (double-precision)") (InputAction :type "InputAction Object Reference" :default "/Game/shooting_game/Input/IA_Restart.IA_Restart"))
  (:`Triggered`
    (`GameplayStatics.OpenLevel` "Level1")))

(event `DieEvnet`
  (bind _returnvalue (pcsubsystem `EnhancedInputLocalPlayerSubsystem` (`GameplayStatics.GetPlayerController` 0)))
  (bind _returnvalue_2 (`|CreateWidget` "/Game/shooting_game/UI/WBP_GameOver.WBP_GameOver_C"))
  (`UserWidget.AddToViewport` _returnvalue_2 0)
  (message `EnhancedInputSubsystemInterface.RemoveMappingContext` _returnvalue "/Game/shooting_game/Input/IMC_Fighter.IMC_Fighter" (struct))
  (`KismetSystemLibrary.Delay` 0.1)
  (message `EnhancedInputSubsystemInterface.AddMappingContext` _returnvalue "/Game/shooting_game/Input/IMC_Menu.IMC_Menu" 1 (struct)))

(fn `GetHealth`
  (returns (CurrentHealth :type "Float (double-precision)"))
  (return (`self.PlayerHealth`)))

(fn `GetMaxHealth`
  (returns (MaxHealth :type "Float (double-precision)"))
  (return (`self.PlayerMaxHealth`)))

(fn `UserConstructionScript`)