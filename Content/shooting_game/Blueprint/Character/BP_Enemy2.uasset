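; BP_Enemy2 is a shooting-game enemy that weaves sideways while firing and removes itself after a fixed lifetime.
; On BeginPlay a looping timer spawns BP_EnemyBullet from the skeletal mesh's transform at the configured fire rate.
; A timeline wave scaled by Width offsets the mesh along its relative right axis, and its Update also starts the delayed destroy.
; An older Y-bound actor movement branch remains unconnected.
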(event `self.ReceiveTick`
  (params (DeltaSeconds :type "Float (single-precision)")))

(event `self.ReceiveBeginPlay`
  (`KismetSystemLibrary.K2_SetTimerDelegate` (delegate `ShootingBullet`) (`self.ShootRate`) true)
  (bind (_direction _wave) (`Timeline|타임라인` :!via `PlayFromStart`)
    (:`Update`
      (`SceneComponent.K2_SetRelativeLocation` (`self.SkeletalMesh`) (* _wave (`self.Width`) (`KismetMathLibrary.Vector_Right`)) false false)
      (`KismetSystemLibrary.Delay` 30.0)
      (`self.K2_DestroyActor`))))

(event `ShootingBullet`
  (`|SpawnActorFromClass` "/Game/shooting_game/Blueprint/SubObject/BP_EnemyBullet.BP_EnemyBullet_C" (`SceneComponent.K2_GetComponentToWorld` (`self.SkeletalMesh`)) "Undefined" "MultiplyWithRoot" null null))

(fn `UserConstructionScript`
  (`parent.UserConstructionScript`))