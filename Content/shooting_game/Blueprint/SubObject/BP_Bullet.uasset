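; BP_Bullet is a shooter projectile that damages what it overlaps and removes itself afterward.
; On overlap it ignores actors tagged Player or Bullet, applies BulletDamage to anything else, then calls its Destroy event.
; A timer started at BeginPlay calls the same Destroy event after LifeTime, so expiry and impact both spawn the hit particle system before the actor is destroyed.
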(event `self.ReceiveBeginPlay`
  (`KismetSystemLibrary.K2_SetTimerDelegate` (delegate `Destroy`) (`self.LifeTime`)))

(event `Destroy`
  (`NiagaraFunctionLibrary.SpawnSystemAtLocation` (`self.HitParticle`) (`self.K2_GetActorLocation`))
  (`self.K2_DestroyActor`))

(event `self.ReceiveActorBeginOverlap`
  (params (OtherActor :type "Actor Object Reference"))
  (if (not (or (`self.ActorHasTag` OtherActor "Player") (`self.ActorHasTag` OtherActor "Bullet")))
    (`GameplayStatics.ApplyDamage` OtherActor (`self.BulletDamage`))
    (`self.Destroy`)))

(fn `UserConstructionScript`)