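; BP_ObjectPool is an object pool actor for bullets in a shooting game, toggling visibility and collision.
; On BeginPlay it spawns BulletClass actors at its root transform, counted by PoolSize, hidden and without collision, but never adds them to PoolBullets.
; ActivateBullet loops over PoolBullets without breaking, showing and enabling collision wherever the Hidden check passes.
; DeactivateBullet hides the given bullet and disables its collision instead of destroying it.
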(event `self.ReceiveBeginPlay`
  (for _ (range (+ (- (`self.PoolSize`) -1) 1))
    (bind _returnvalue (`|SpawnActorFromClass` (`self.BulletClass`) (`SceneComponent.K2_GetComponentToWorld` (`self.DefaultSceneRoot`)) "Undefined" "MultiplyWithRoot" null null))
    (`self.SetActorHiddenInGame` _returnvalue true)
    (`self.SetActorEnableCollision` _returnvalue false)))

(event `ActivateBullet`
  (for _array_element (`self.PoolBullets`)
    (if (`self.bHidden`)
      (`self.SetActorHiddenInGame` _array_element false)
      (`self.SetActorEnableCollision` _array_element true))))

(event `DeactivateBullet`
  (params (Bullet :type "/Game/shooting_game/Blueprint/SubObject/BP_Bullet Object Reference"))
  (`self.SetActorHiddenInGame` Bullet true)
  (`self.SetActorEnableCollision` Bullet false))

(fn `UserConstructionScript`)