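; BP_EnemyBullet is an enemy projectile Blueprint for a shooting game that damages what it hits.
; On actor overlap it ignores anything tagged Bullet or Enemy, so shots pass through each other and through enemies.
; For any other actor it applies its BulletDamage value and destroys itself.
; BeginPlay and the construction script only call their parent versions.
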(event `self.ReceiveBeginPlay`
  (`parent.ReceiveBeginPlay`))

(event `self.ReceiveActorBeginOverlap`
  (params (OtherActor :type "Actor Object Reference"))
  (if (not (or (`self.ActorHasTag` OtherActor "Bullet") (`self.ActorHasTag` OtherActor "Enemy")))
    (`GameplayStatics.ApplyDamage` OtherActor (`self.BulletDamage`))
    (`self.Destroy`)))

(fn `UserConstructionScript`
  (`parent.UserConstructionScript`))