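; Bomb projectile for the shooting game that deals radial damage on contact.
; When its sphere overlaps an actor not tagged Player or Bullet, it applies full, falloff-free damage within the bomb radius, then calls Destroy.
; A lifetime timer started at BeginPlay spawns the hit particle system and destroys the actor, without applying damage.
; Parent BeginPlay and overlap calls are disconnected, so that inherited Blueprint logic does not run.
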(event `self.ReceiveBeginPlay`
  (`KismetSystemLibrary.K2_SetTimerDelegate` (delegate `CustomEvent`) (`self.LifeTime`)))

(event `CustomEvent`
  (`NiagaraFunctionLibrary.SpawnSystemAtLocation` (`self.HitParticle`) (`self.K2_GetActorLocation`))
  (`self.K2_DestroyActor`))

(event `self.Sphere1.OnComponentBeginOverlap`
  (params (OverlappedComponent :type "PrimitiveComponent Object Reference") (OtherActor :type "Actor Object Reference") (OtherComp :type "PrimitiveComponent Object Reference") (OtherBodyIndex :type Integer) (bFromSweep :type Boolean) (SweepResult :type "HitResult Structure (by ref)"))
  (if (not (or (`self.ActorHasTag` OtherActor "Player") (`self.ActorHasTag` OtherActor "Bullet")))
    (bind _returnvalue (`GameplayStatics.ApplyRadialDamage` :`BaseDamage` (`self.BombDamage`) :`Origin` (`self.K2_GetActorLocation`) :`DamageRadius` (`self.BombRadius`) :`DamageCauser` null :`InstigatedByController` null :`bDoFullDamage` true))
    (`self.Destroy`)))

(event `self.ReceiveActorBeginOverlap`
  (params (OtherActor :type "Actor Object Reference")))

(fn `UserConstructionScript`
  (`parent.UserConstructionScript`))